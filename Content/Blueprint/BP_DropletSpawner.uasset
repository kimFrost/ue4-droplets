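; BP_DropletSpawner is an actor that scatters 300 BP_Droplet actors in random colours over a wide square area around itself.
; Its construction script adds each droplet as a Child Actor Component at a random horizontal offset and height band, with no active event graph logic.
; Each droplet receives one of six preset colours at random, then UpdateColor is called on it.
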(fn `UserConstructionScript`
  (bind _returnvalue (* 8000.0 -1.0))
  (for _ (range 300)
    (bind _returnvalue_2 (`AddComponent|NODE_AddChildActorComponent-0` :`RelativeTransform` (`KismetMathLibrary.MakeTransform` (`KismetMathLibrary.MakeVector` (`KismetMathLibrary.RandomFloatInRange` _returnvalue 8000.0) (`KismetMathLibrary.RandomFloatInRange` _returnvalue 8000.0) (`KismetMathLibrary.RandomFloatInRange` 150.0 400.0)) (struct) (1.0 1.0 1.0))))
    (`ChildActorComponent.SetChildActorClass` _returnvalue_2 "/Game/Blueprint/BP_Droplet.BP_Droplet_C")
    (bind _asbp_droplet (cast `/Game/Blueprint/BP_Droplet` (`ChildActorComponent.ChildActor` _returnvalue_2)))
    (set `/Game/Blueprint/BP_Droplet.Color` (select `int` (`KismetMathLibrary.RandomIntegerInRange` 0 5) :`0` (struct :`G` 1.0 :`B` 0.812248 :`A` 1.0) :`1` (struct :`R` 1.0 :`B` 0.933825 :`A` 1.0) :`2` (struct :`R` 0.452964 :`G` 1.0 :`A` 1.0) :`3` (struct :`R` 1.0 :`G` 0.853497 :`A` 1.0) :`4` (struct :`R` 1.0 :`B` 0.054682 :`A` 1.0) :`5` (struct :`G` 0.123196 :`B` 1.0 :`A` 1.0) :!type "LinearColor Structure") _asbp_droplet)
    (`/Game/Blueprint/BP_Droplet.UpdateColor` _asbp_droplet)))